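; Drink glass actor for the Barman game that tracks a fill amount and shows it as a liquid level and text label.
; The construction script sets the label and creates a dynamic coffee-fill material on the cylinder.
; AddFill clamps the total between empty and full, updates the label and drives the material's fill height with a centered offset.
; The label switches to the overfill color once the glass is full.
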(fn `AddFill`
  (params (Amount :type "Float (double-precision)"))
  (bind _fillamountlabel (`self.FillAmountLabel`))
  (bind _output_get (set `self.FillAmount` (`KismetMathLibrary.FClamp` (+ (`self.FillAmount`) Amount))))
  (`TextRenderComponent.K2_SetText` _fillamountlabel (`KismetTextLibrary.Conv_DoubleToText` _output_get "HalfToEven"))
  (`MaterialInstanceDynamic.SetScalarParameterValue` (`self.Fill Material`) "Liquid_FillHeight" (- _output_get 0.5))
  (if (>= (`self.FillAmount`) 1.0)
    (`TextRenderComponent.SetTextRenderColor` _fillamountlabel (`self.OverFillColor`))))

(fn `UserConstructionScript`
  (`TextRenderComponent.K2_SetText` (`self.FillAmountLabel`) (`KismetTextLibrary.Conv_DoubleToText` (`self.FillAmount`) "HalfToEven"))
  (bind _returnvalue (`PrimitiveComponent.CreateDynamicMaterialInstance` (`self.Cylinder`) 0 "/Game/LiquidMaterials/Materials/MI_CoffeeFill.MI_CoffeeFill" "None"))
  (set `self.Fill Material` _returnvalue))