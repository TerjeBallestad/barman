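; BP_DrinkPitcher is a drink pitcher for the Barman game that tracks how full it is and displays that amount on a label.
; AddFill adds an amount to DrinkAmount, clamps the result between empty and full, and refreshes FillAmountLabel.
; The construction script sets the label from the starting amount.
; BeginPlay stores the root's world location as InitialLocation, which nothing else in these graphs reads.
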(event `self.ReceiveBeginPlay`
  (set `self.InitialLocation` (`SceneComponent.K2_GetComponentLocation` (`self.DefaultSceneRoot`))))

(event `self.ReceiveTick`
  (params (DeltaSeconds :type "Float (single-precision)")))

(fn `AddFill`
  (params (Amount :type "Float (double-precision)"))
  (bind _output_get (set `self.DrinkAmount` (`KismetMathLibrary.FClamp` (+ Amount (`self.DrinkAmount`)))))
  (`TextRenderComponent.K2_SetText` (`self.FillAmountLabel`) (`KismetTextLibrary.Conv_DoubleToText` _output_get "HalfToEven")))

(fn `UserConstructionScript`
  (`TextRenderComponent.K2_SetText` (`self.FillAmountLabel`) (`KismetTextLibrary.Conv_DoubleToText` (`self.DrinkAmount`) "HalfToEven")))