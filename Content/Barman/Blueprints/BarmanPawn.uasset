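; Player pawn for bartending with the mouse: picks up drink pitchers and pours them into glasses.
; The Grip input toggles holding the BP_DrinkPitcher under the cursor, keeping the grab offset.
; On Tick, cursor traces against BP_BarBoundary give a plane-constrained target the pitcher lerps toward, tilting as it rises.
; Past a minimum angle the pitcher drains, and a downward trace from its drip point fills any BP_DrinkGlass hit.
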(event `self.ReceiveBeginPlay`
  (bind _output_get (set `self.PlayerController` (`GameplayStatics.GetPlayerController` 0)))
  (set `PlayerController.bShowMouseCursor` true _output_get))

(event `InputAction|Grip`
  (params (Key :type "Key Structure"))
  (bind _hitresult (`PlayerController.GetHitResultUnderCursorByChannel` (`self.PlayerController`) "TraceTypeQuery1" true))
  ;[1 1 1] Grip Drink Pitcher
  (:`Pressed`
    (`KismetSystemLibrary.PrintString` "clicking")
    (if (`KismetSystemLibrary.IsValid` (`self.PitcherInHand`))
      (`self.ReleaseDrinkPitcher`)
      (else
        (`KismetSystemLibrary.PrintString` (`KismetSystemLibrary.GetDisplayName` (`.HitActor` (`GameplayStatics.BreakHitResult` _hitresult))))
        (bind _asbp_drink_pitcher (cast `/Game/Barman/Blueprints/BP_DrinkPitcher` (`.HitActor` (`GameplayStatics.BreakHitResult` _hitresult))))
        (set `self.PitcherInHand` _asbp_drink_pitcher)
        (`self.GripDrinkPitcher`)
        (bind _output_get (set `self.InitialMouseLocation` (`.Location` (`GameplayStatics.BreakHitResult` _hitresult))))
        (set `self.PitcherOffset` (- (`self.K2_GetActorLocation` (`self.PitcherInHand`)) _output_get))))))

(event `self.ReceiveTick`
  (params (DeltaSeconds :type "Float (single-precision)"))
  (bind _returnvalue (`GameplayStatics.GetWorldDeltaSeconds`))
  (bind _pitcherinhand (`self.PitcherInHand`))
  (bind (_pitcheroffset_x _pitcheroffset_y _pitcheroffset_z) (`KismetMathLibrary.BreakVector` (`self.PitcherOffset`)))
  (bind _pitcherinhand_2 (`self.PitcherInHand`))
  (bind _pitcherinhand_3 (`self.PitcherInHand`))
  (bind (_returnvalue_x _returnvalue_y _returnvalue_z) (`KismetMathLibrary.BreakVector` (`self.K2_GetActorLocation` _pitcherinhand_2)))
  (bind _hitresult (`PlayerController.GetHitResultUnderCursorByChannel` (`self.PlayerController`) "TraceTypeQuery3" false))
  (bind (_initiallocation_x _initiallocation_y _initiallocation_z) (`KismetMathLibrary.BreakVector` (`/Game/Barman/Blueprints/BP_DrinkPitcher.InitialLocation` _pitcherinhand_2)))
  (bind _returnvalue_2 (`SceneComponent.K2_GetComponentLocation` (`/Game/Barman/Blueprints/BP_DrinkPitcher.DripPoint` _pitcherinhand_3)))
  (bind _returnvalue_3 (`KismetMathLibrary.FClamp` (* (- _returnvalue_z _initiallocation_z) (`self.PitcherRotationMultiplier`)) 0.0 (`self.PitcherMaxAngle`)))
  ;[1 1 1] Move Drink Pitcher
  (if (`self.ShouldMovePitcher`)
    (if (!= (`self.PitcherDestination`) (0.0 0.0 0.0))
      (`self.K2_SetActorLocation` _pitcherinhand (`KismetMathLibrary.VLerp` (`self.K2_GetActorLocation` _pitcherinhand) (`self.PitcherDestination`) 0.1) true false))
    (bind _asbp_bar_boundary (cast `/Game/Barman/Blueprints/BP_BarBoundary` (`.HitActor` (`GameplayStatics.BreakHitResult` _hitresult))))
    (bind _outlocation (`/Game/Barman/Blueprints/BP_BarBoundary.GetClosesLocationOnMovablePlane` _asbp_bar_boundary (+ (`.Location` (`GameplayStatics.BreakHitResult` _hitresult)) (`KismetMathLibrary.MakeVector` _pitcheroffset_x 0.0 _pitcheroffset_z))))
    (set `self.PitcherDestination` _outlocation)
    ;[1 1 1] Rotate drink pitcher
    (`self.K2_SetActorRotation` _pitcherinhand_2 (`KismetMathLibrary.MakeRotator` 0.0 _returnvalue_3) false)
    ;[1 1 1] Check if should pour drink
    (if (> _returnvalue_3 (`self.MinimumDrippingAngle`))
      ;[1 1 1] Pour Drink
      (`/Game/Barman/Blueprints/BP_DrinkPitcher.AddFill` _pitcherinhand_3 (* _returnvalue -0.1))
      (bind _outhit (`KismetSystemLibrary.LineTraceSingle` _returnvalue_2 (+ _returnvalue_2 (0.0 0.0 -200.0)) "TraceTypeQuery1" false (`self.Actors to Ignore`) "ForOneFrame"))
      (bind _asbp_drink_glass (cast `/Game/Barman/Blueprints/BP_DrinkGlass` (`.HitActor` (`GameplayStatics.BreakHitResult` _outhit))))
      (`/Game/Barman/Blueprints/BP_DrinkGlass.AddFill` _asbp_drink_glass (* _returnvalue 0.5)))))

(fn `GripDrinkPitcher`
  (bind _pitcherinhand (`self.PitcherInHand`))
  (`KismetSystemLibrary.PrintString` "Gripping pitcher")
  (set `PlayerController.bShowMouseCursor` true (`self.PlayerController`))
  (set `self.ShouldMovePitcher` true)
  (set `/Game/Barman/Blueprints/BP_DrinkPitcher.InitialLocation` (`self.K2_GetActorLocation` _pitcherinhand) _pitcherinhand))

(fn `ReleaseDrinkPitcher`
  (`KismetSystemLibrary.PrintString` "Releasing pitcher")
  (set `self.PitcherInHand` null)
  (set `PlayerController.bShowMouseCursor` true (`self.PlayerController`))
  (set `self.ShouldMovePitcher` false))

(fn `UserConstructionScript`)